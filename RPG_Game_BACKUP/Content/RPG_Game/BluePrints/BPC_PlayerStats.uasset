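; Actor component that tracks the RPG hero's health and stamina, caching its BP_Hero owner on BeginPlay.
; Decrease functions subtract and return true at zero or below, while increase functions cap at the maximum.
; Health changes push a percentage to the hero's HUD health bar; stamina changes do not update the HUD.
; IncreaseMaxHealth derives the new maximum from current health, unlike IncreaseMaxStamina, which adds to the existing maximum.
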(event `self.ReceiveBeginPlay`
  (bind _asbp_hero (cast `/Game/RPG_Game/MainCharacter/RPB_CharacterBP/BP_Hero` (`self.GetOwner`)))
  (set `self.Player Character BP` _asbp_hero))

(fn `Decrease Health`
  (params (Damage :type "Float (double-precision)"))
  (returns (`Is PlayerDead` :type Boolean))
  (bind _output_get (set `self.CurrentHealth` (- (`self.CurrentHealth`) Damage)))
  (`ProgressBar.SetPercent` (`/Game/RPG_Game/RPG_UI/WB_HUD.HealthBar` (`/Game/RPG_Game/MainCharacter/RPB_CharacterBP/BP_Hero.HUD Widget` (`self.Player Character BP`))) (/ _output_get (`self.MaxHealth`)))
  (if (<= (`self.CurrentHealth`) 0.0)
    (return true)
    (else
      (return false))))

(fn `Decrease Stamina`
  (params (`Stamina Depleation` :type "Float (double-precision)"))
  (returns (`No Stamina Left` :type Boolean))
  (set `self.CurrentStamina` (- (`self.CurrentStamina`) `Stamina Depleation`))
  (if (<= (`self.CurrentStamina`) 0.0)
    (return true)
    (else
      (return false))))

(fn `Increase Helth`
  (params (`Added Health` :type "Float (double-precision)"))
  (set `self.CurrentHealth` (+ (`self.CurrentHealth`) `Added Health`))
  (if (> (`self.CurrentHealth`) (`self.MaxHealth`))
    (set `self.CurrentHealth` (`self.MaxHealth`)))
  (`ProgressBar.SetPercent` (`/Game/RPG_Game/RPG_UI/WB_HUD.HealthBar` (`/Game/RPG_Game/MainCharacter/RPB_CharacterBP/BP_Hero.HUD Widget` (`self.Player Character BP`))) (/ (`self.CurrentHealth`) (`self.MaxHealth`))))

(fn `Increase Max Health`
  (params (`Health Incriments` :type "Float (double-precision)"))
  (set `self.MaxHealth` (+ (`self.CurrentHealth`) `Health Incriments`))
  (`ProgressBar.SetPercent` (`/Game/RPG_Game/RPG_UI/WB_HUD.HealthBar` (`/Game/RPG_Game/MainCharacter/RPB_CharacterBP/BP_Hero.HUD Widget` (`self.Player Character BP`))) (/ (`self.CurrentHealth`) (`self.MaxHealth`))))

(fn `Increase Max Stamina`
  (params (`Add Stamina` :type "Float (double-precision)"))
  (set `self.MaxStamina` (+ (`self.MaxStamina`) `Add Stamina`)))

(fn `Increase Stamina`
  (params (`Added Stamina` :type "Float (double-precision)"))
  (set `self.CurrentStamina` (+ (`self.CurrentStamina`) `Added Stamina`))
  (if (> (`self.CurrentStamina`) (`self.MaxStamina`))
    (set `self.CurrentStamina` (`self.MaxStamina`))))